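; Base character Blueprint that sets up the player's main HUD and provides debug shortcuts for camera distance and slow motion.
; On BeginPlay it creates WBP_MainHud for the owning player controller and adds it to the viewport, skipping this if the controller is not a PlayerController.
; Debug key B flip-flops the spring arm between near and far lengths, and holding the second thumb mouse button slows global time dilation until release.
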(event EventBeginPlay
  (bind _asplayer_controller (Utilities|Casting|CastToPlayerController (Pawn|GetController)))
  (bind _returnvalue (UserInterface|CreateWidget "/Game/Blueprints/WBP_MainHud.WBP_MainHud_C" _asplayer_controller))
  (UserInterface|Viewport|AddtoViewport _returnvalue 0))

(event Collision|EventActorBeginOverlap
  (params (OtherActor :type Actor%20Object%20Reference)))

(event EventTick
  (params (DeltaSeconds :type Float%20%28single-precision%29)))

(event Input|KeyboardEvents|DebugKeyB
  (params (Key :type Key%20Structure :default "None") (ActionValue :type Input%20Action%20Value%20Structure))
  (bind _springarmcomponent (Variables|Default|GetSpringArmComponent))
  (:Pressed
    (Utilities|FlowControl|FlipFlop
      (:A
        (Variables|/Script/Engine.SpringArmComponent|SetTargetArmLength _springarmcomponent 2e+02))
      (:B
        (Variables|/Script/Engine.SpringArmComponent|SetTargetArmLength _springarmcomponent 1e+03)))))

(event Input|MouseEvents|DebugKeyThumbMouseButton2
  (params (Key :type Key%20Structure :default "None") (ActionValue :type Input%20Action%20Value%20Structure))
  (:Pressed
    (Utilities|Time|SetGlobalTimeDilation 0.1))
  (:Released
    (Utilities|Time|SetGlobalTimeDilation 1.0)))

(fn ConstructionScript)